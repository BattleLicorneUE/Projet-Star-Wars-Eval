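; Combat manager, likely an AI component, that runs special melee, combo melee and ranged attacks one at a time.
; Each attack passes an IsAttacking gate and DoOnce, then plays its montage through a macro that releases the lock afterwards.
; Combos advance through a montage array, with the index reset by a retriggerable delay.
; Ranged attacks fire a projectile at player 0's position on an anim notify.
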(event `LaunchOnlyOneAttack`
  (params (Target :type "Character Object Reference") (S_DataAI :type "/Game/StarWarsCore/IA/Data/S_DataAI Structure (by ref)"))
  (`self.CanAttack?`
    (:`True`
      (`/Engine/EditorBlueprintResources/StandardMacros.DoOnce` false :!label _label
        (:`Completed`
          (`self.AnimMelee` Target S_DataAI)
          (set `self.IsAttacking` false)
          (goto _label :!via `Reset`))))))

(event `LaunchRangeAttack`
  (params (Mesh :type "SkeletalMeshComponent Object Reference") (`Spawn Transform Location` :type "Vector Structure"))
  (`self.CanAttack?`
    (:`True`
      (`/Engine/EditorBlueprintResources/StandardMacros.DoOnce` false :!label _label_2
        (:`Completed`
          (`self.AnimRange` Mesh
            (:`On Blend Out`
              (set `self.IsAttacking` false)
              (`self.SpawnProjectile` `Spawn Transform Location`)
              (goto _label_2 :!via `Reset`))))))))

(event `LaunchAttack`
  (params (S_Data :type "/Game/StarWarsCore/IA/Data/S_DataAI Structure") (Character :type "/Game/StarWarsCore/Blueprints/Characters/NPC/BP_Base_NPC Object Reference"))
  (`self.CanAttack?`
    (:`True`
      (`/Engine/EditorBlueprintResources/StandardMacros.DoOnce` false :!label _label_3
        (:`Completed`
          (`self.AnimMeleeCombo` S_Data Character
            (:`On Blend Out`
              (set `self.IsAttacking` false)
              (`|ExecutionSequence`
                (:`then_0`
                  (goto _label_3 :!via `Reset`))
                (:`then_1`
                  (`KismetSystemLibrary.RetriggerableDelay` 5.0)
                  (set `self.Index` 0))))))))))

(fn `SpawnProjectile`
  (params (`Spawn Transform Location` :type "Vector Structure"))
  (`|SpawnActorFromClass` "/Game/StarWarsCore/Blueprints/Actors/Projectile/BP_Projectile.BP_Projectile_C" (`KismetMathLibrary.MakeTransform` `Spawn Transform Location` (`KismetMathLibrary.FindLookAtRotation` `Spawn Transform Location` (`Actor.K2_GetActorLocation` (`GameplayStatics.GetPlayerCharacter` 0)))) "Undefined" "MultiplyWithRoot" null null))