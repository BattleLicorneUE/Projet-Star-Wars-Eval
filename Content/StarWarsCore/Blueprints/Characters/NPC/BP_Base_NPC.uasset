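; Base NPC Blueprint that switches its AI state when its perception component reports the player.
; It stores its spawn location as InitialPosition on BeginPlay.
; A perception update targeting player character 0 prints a debug "see", sets the StateAI enum and writes it to the Blackboard.
; The handler does not check whether the player was sensed or lost, and never switches the state back.
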(event `self.ReceiveBeginPlay`
  (`parent.ReceiveBeginPlay`)
  (set `self.InitialPosition` (`self.K2_GetActorLocation`)))

(event `self.AIPerception.OnTargetPerceptionInfoUpdated`
  (params (UpdateInfo :type "ActorPerceptionUpdateInfo Structure (by ref)"))
  (if (== (`.Target` (break `ActorPerceptionUpdateInfo` UpdateInfo)) (`GameplayStatics.GetPlayerCharacter` 0))
    (`KismetSystemLibrary.PrintString` "see" true true (struct :`R` 1.0 :`G` 0.151505 :`B` 0.009725 :`A` 1.0) 0.1)
    (bind _output_get (set `self.StateAI` "NewEnumerator2"))
    (`BlackboardComponent.SetValueAsEnum` (`AIBlueprintHelperLibrary.GetBlackboard` null) "StateAI" _output_get)))

(fn `UserConstructionScript`
  (`parent.UserConstructionScript`))