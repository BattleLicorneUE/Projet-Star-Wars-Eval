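; BP_Boss_Child is a Star Wars NPC boss character that fights with a red lightsaber.
; On BeginPlay it sets the saber child actor to BP_BaseSaber and turns it red.
; Every tick it updates a Motion Warping "Target" to the player's location and facing yaw.
; Melee, ranged and special attack events delegate to the ACCombatAIManager component, while a separate AnimMelee graph plays a melee montage.
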(event `self.ReceiveBeginPlay`
  (`parent.ReceiveBeginPlay`)
  (`ChildActorComponent.SetChildActorClass` (`self.ChildActor_Saber`) "/Game/StarWarsCore/Blueprints/Actors/Weapons/BP_BaseSaber.BP_BaseSaber_C")
  (bind _asbp_base_saber (cast `/Game/StarWarsCore/Blueprints/Actors/Weapons/BP_BaseSaber` (`ChildActorComponent.ChildActor` (`self.ChildActor_Saber`))))
  (`/Game/StarWarsCore/Blueprints/Actors/Weapons/BP_BaseSaber.ChangeColorToRed` _asbp_base_saber))

(event `self.ReceiveTick`
  (params (DeltaSeconds :type "Float (single-precision)"))
  (bind _returnvalue (`self.K2_GetActorLocation` (`GameplayStatics.GetPlayerCharacter` 0)))
  (`parent.ReceiveTick` DeltaSeconds)
  (`MotionWarpingComponent.AddOrUpdateWarpTargetFromLocationAndRotation` (`self.MotionWarping`) "Target" _returnvalue (`KismetMathLibrary.MakeRotator` 0.0 0.0 (.yaw (`KismetMathLibrary.FindLookAtRotation` (`self.K2_GetActorLocation`) _returnvalue)))))

(event `AttackMelee`
  (`/Game/StarWarsCore/IA/AC_CombatAIManager.LaunchAttack` (`self.AC_CombatAIManager`) (`self.S_Data`) self))

(event `AttackRange`
  (`/Game/StarWarsCore/IA/AC_CombatAIManager.LaunchRangeAttack` (`self.AC_CombatAIManager`) (`self.Mesh`) (`self.K2_GetActorLocation`) self))

(event `AttackSpecial`
  (`/Game/StarWarsCore/IA/AC_CombatAIManager.LaunchOnlyOneAttack` (`self.AC_CombatAIManager`) self (`self.S_Data`)))

(fn `UserConstructionScript`
  (`parent.UserConstructionScript`))