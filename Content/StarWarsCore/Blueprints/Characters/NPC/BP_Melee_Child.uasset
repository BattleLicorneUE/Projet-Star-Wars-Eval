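; Melee NPC child Blueprint in the Star Wars core content that fights with a red saber.
; On BeginPlay it sets the ChildActorSaber class from BaseSaber, then turns the spawned BP_BaseSaber red.
; The Attack event hands SData and itself to the combat AI manager component's LaunchAttack.
; An AttackAnim function plays a melee montage, but its only call in the event graph is unconnected.
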(event `self.ReceiveBeginPlay`
  (`parent.ReceiveBeginPlay`)
  (`ChildActorComponent.SetChildActorClass` (`self.ChildActor_Saber`) (`self.BaseSaber`))
  (bind _asbp_base_saber (cast `/Game/StarWarsCore/Blueprints/Actors/Weapons/BP_BaseSaber` (`ChildActorComponent.ChildActor` (`self.ChildActor_Saber`))))
  (`/Game/StarWarsCore/Blueprints/Actors/Weapons/BP_BaseSaber.ChangeColorToRed` _asbp_base_saber))

(event `Attack`
  (`/Game/StarWarsCore/IA/AC_CombatAIManager.LaunchAttack` (`self.AC_CombatAIManager`) (`self.S_Data`) self))

(fn `UserConstructionScript`
  (`parent.UserConstructionScript`))