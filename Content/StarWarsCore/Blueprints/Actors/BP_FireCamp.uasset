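; BP_FireCamp is a campfire actor that records level NPCs so they can be respawned.
; On BeginPlay it stores the class and location of every BP_Base_NPC actor in a map.
; Respawn spawns an actor for each map entry at its saved location, without removing existing NPCs.
; Because the map is keyed by class, only the last recorded position per NPC class is kept.
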(event `self.ReceiveBeginPlay`
  (bind _outactors (`GameplayStatics.GetAllActorsOfClass` "/Game/StarWarsCore/Blueprints/Characters/NPC/BP_Base_NPC.BP_Base_NPC_C"))
  (for _array_element _outactors
    (`BlueprintMapLibrary.Map_Add` (`self.ClassAndPosition`) (`GameplayStatics.GetObjectClass` _array_element) (`self.K2_GetActorLocation` _array_element))))

(fn `Respawn`
  (bind _keys (`BlueprintMapLibrary.Map_Keys` (`self.ClassAndPosition`)))
  (for (_array_element _array_index) _keys
    (bind _values (`BlueprintMapLibrary.Map_Values` (`self.ClassAndPosition`)))
    (`|SpawnActorFromClass` _array_element (`KismetMathLibrary.MakeTransform` (`|GetArrayItem` _values _array_index)) "Undefined" "MultiplyWithRoot" null (struct) null)))

(fn `UserConstructionScript`)