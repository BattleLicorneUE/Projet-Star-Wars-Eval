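; BP_BaseSaber is the base saber weapon, handling melee hit detection and damage between the player and NPCs.
; Raycast sphere-traces between two blade points, ignoring the attach parent, and checks each hit.
; NPC-owned sabers reduce player stats when CanDamage is set; separately, hit NPCs take the player's force-based damage, gated by CanBeDamaged.
; Both gates clear upon a hit, and ChangeColorToRed swaps the blade material.
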(fn `ChangeColorToRed`
  (`PrimitiveComponent.SetMaterial` (`self.SM_Blade`) 0 "/Game/StarWarsCore/Resources/Materials/Base/MI_Light_Red.MI_Light_Red"))

(fn `Raycast`
  (bind _returnvalue (`GameplayStatics.GetPlayerCharacter` 0))
  (bind (_outhits _returnvalue_2) (`KismetSystemLibrary.SphereTraceMultiForObjects` (`SceneComponent.K2_GetComponentLocation` (`self.Raycast_Start`)) (`SceneComponent.K2_GetComponentLocation` (`self.Raycast_End`)) 25.0 (`|MakeArray` "ObjectTypeQuery3" "ObjectTypeQuery1" :!type "EObjectTypeQuery Enum") false (`|MakeArray` (`self.GetAttachParentActor`))))
  (if _returnvalue_2
    (for _array_element _outhits
      (`|ExecutionSequence`
        (:`then_0`
          (bind _asbp_base_npc (cast `/Game/StarWarsCore/Blueprints/Characters/NPC/BP_Base_NPC` (`self.GetParentActor`)))
          (bind _returnvalue_3 (`self.GetComponentByClass` _asbp_base_npc "/Game/StarWarsCore/IA/AC_CombatAIManager.AC_CombatAIManager_C"))
          (if (`/Game/StarWarsCore/IA/AC_CombatAIManager.CanDamage` _returnvalue_3)
            (bind (_bblockinghit _binitialoverlap _time _distance _location _impactpoint _normal _impactnormal _physmat _hitactor) (`GameplayStatics.BreakHitResult` _array_element))
            (bind _asbp_player_character (cast `/Game/StarWarsCore/Blueprints/Characters/BP_PlayerCharacter` _hitactor))
            (set `/Game/StarWarsCore/IA/AC_CombatAIManager.CanDamage` false _returnvalue_3)
            (bind _damage (message `/Game/StarWarsCore/IA/BI_AI.ApplyDamage` _asbp_base_npc))
            (`KismetSystemLibrary.PrintString` (`KismetStringLibrary.Conv_DoubleToString` _damage))
            (message `/Game/StarWarsCore/Blueprints/ActorsComponents/ManagerStats/BPI_Stats.ModifyCurrentPv` (`self.GetComponentByClass` _asbp_player_character "/Game/StarWarsCore/Blueprints/ActorsComponents/ManagerStats/AC_Stats.AC_Stats_C") _damage false)))
        (:`then_1`
          (if (`Actor.bCanBeDamaged` _returnvalue)
            (bind _asbp_base_npc_2 (cast `/Game/StarWarsCore/Blueprints/Characters/NPC/BP_Base_NPC` _hitactor))
            (set `Actor.bCanBeDamaged` false _returnvalue)
            (bind _damage_2 (`/Game/StarWarsCore/Blueprints/ActorsComponents/ManagerStats/AC_Stats.ApplyDamageWithForce` (`self.GetComponentByClass` _returnvalue "/Game/StarWarsCore/Blueprints/ActorsComponents/ManagerStats/AC_Stats.AC_Stats_C")))
            (message `/Game/StarWarsCore/IA/BI_AI.TakeDamage` _asbp_base_npc_2 _damage_2)
            (`KismetSystemLibrary.PrintString` (`KismetStringLibrary.Conv_DoubleToString` _damage_2))))))))

(fn `UserConstructionScript`)