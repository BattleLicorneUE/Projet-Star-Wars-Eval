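; BP_Trigger_Blend_Camera is a one-shot trigger actor that briefly shows a cinematic camera view when the player character enters it.
; On first overlap with BP_PlayerCharacter, it disables player input and blends the view to the assigned Camera.
; After a short hold, it eases the view back to the player and re-enables input once that blend finishes.
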(event `self.ReceiveActorBeginOverlap`
  (params (OtherActor :type "Actor Object Reference"))
  (cast `/Game/StarWarsCore/Blueprints/Characters/BP_PlayerCharacter` OtherActor)
  (`/Engine/EditorBlueprintResources/StandardMacros.DoOnce` false
    (:`Completed`
      (`self.Camera`
        (:`then`
          (`self.DisableInput` (`GameplayStatics.GetPlayerCharacter` 0) (`GameplayStatics.GetPlayerController` 0))
          (`PlayerController.SetViewTargetWithBlend` (`GameplayStatics.GetPlayerController` 0) (`self.Camera`) (`self.Blend Time In`) "VTBlend_Linear" 0.0 false)
          (`KismetSystemLibrary.Delay` (+ (`self.Blend Time In`) 0.5))
          (`PlayerController.SetViewTargetWithBlend` (`GameplayStatics.GetPlayerController` 0) (`GameplayStatics.GetPlayerCharacter` 0) (`self.Blend Time Out`) "VTBlend_EaseIn" 0.0 false)
          (`KismetSystemLibrary.Delay` (`self.Blend Time Out`))
          (`self.EnableInput` (`GameplayStatics.GetPlayerCharacter` 0) (`GameplayStatics.GetPlayerController` 0)))
        (:`else`)))))

(fn `UserConstructionScript`)