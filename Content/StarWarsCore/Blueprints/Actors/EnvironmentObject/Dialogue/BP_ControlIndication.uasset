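; BP_ControlIndication is a one-shot trigger actor that shows the player how to heal, noted by its author as a slightly dirty solution.
; When a BP_PlayerCharacter enters its detection zone, it creates a WB_HowToHeal widget for the first player controller and adds it to the viewport.
; After a configurable duration, it removes the widget and destroys itself, with no guard against repeat overlaps during the delay.
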(event `self.DetectionZone_0.OnComponentBeginOverlap`
  (params (OverlappedComponent :type "PrimitiveComponent Object Reference") (OtherActor :type "Actor Object Reference") (OtherComp :type "PrimitiveComponent Object Reference") (OtherBodyIndex :type Integer) (bFromSweep :type Boolean) (SweepResult :type "HitResult Structure (by ref)"))
  ;[0.2263 0.2519 1] Moyen un peu sale d'indiquer au joueur comment se soigner
  (cast `/Game/StarWarsCore/Blueprints/Characters/BP_PlayerCharacter` OtherActor)
  (bind _returnvalue (`|CreateWidget` "/Game/StarWarsCore/Blueprints/Actors/EnvironmentObject/Dialogue/WB_HowToHeal.WB_HowToHeal_C" (`GameplayStatics.GetPlayerController` 0)))
  (bind _output_get (set `self.WidgetButtonToHeal` _returnvalue))
  (`UserWidget.AddToViewport` _output_get 0)
  (`KismetSystemLibrary.Delay` (`self.Widget duration`))
  (`Widget.RemoveFromParent` (`self.WidgetButtonToHeal`))
  (set `self.WidgetButtonToHeal` (`self.WidgetButtonToHeal`))
  (`self.K2_DestroyActor`))

(fn `UserConstructionScript`)