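; NPC actor that shows its dialogue lines on screen one at a time, advancing each time its Talk event is called.
; Talk increments an index into the Dialogue array, lazily creates a WB_Dialogue widget, sets its text and plays a 2D sound.
; Once the index passes the last line, the widget is removed from its parent; the index is never reset here.
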(event `/Game/StarWarsCore/Blueprints/Actors/EnvironmentObject/Dialogue/BPI_Dialogues.Talk`
  (`/Engine/EditorBlueprintResources/StandardMacros.IncrementInt` (`self.talkIndex`)
    (:`  `
      (if (< (`self.talkIndex`) (`KismetArrayLibrary.Array_Length` (`self.Dialogue`)))
        (`self.UI`
          (:`then`
            _)
          (:`else`
            (bind _returnvalue (`|CreateWidget` "/Game/StarWarsCore/Blueprints/Actors/EnvironmentObject/Dialogue/WB_Dialogue.WB_Dialogue_C" (`GameplayStatics.GetPlayerController` 0)))
            (bind _output_get (set `self.UI` _returnvalue))
            (`UserWidget.AddToViewport` _output_get 0)))
        (`TextBlock.SetText` (`/Game/StarWarsCore/Blueprints/Actors/EnvironmentObject/Dialogue/WB_Dialogue.TalkText` (`self.UI`)) (`KismetTextLibrary.Conv_StringToText` (`|GetArrayItem` (`self.Dialogue`) (`self.talkIndex`))))
        (`GameplayStatics.PlaySound2D` "/Game/StarWarsCore/Characters/PackAnimations/CLazyAnimpack/Demo/Sound/Wave/Golf_Air_Swing_1.Golf_Air_Swing_1" 1.0 1.0 0.0 null null) ; Ajout un feedback Sonor a chaque texte
        (else
          (`Widget.RemoveFromParent` (`self.UI`)))))))

(fn `UserConstructionScript`)