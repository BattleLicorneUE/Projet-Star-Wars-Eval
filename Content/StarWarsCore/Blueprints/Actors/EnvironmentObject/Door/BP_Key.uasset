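; BP_Key is a key pickup that the player collects to be able to open a door.
; Box overlap by BP_PlayerCharacter shows the WB_PickUp prompt, enables input and opens a Gate; leaving removes the prompt, calls DisableInput and closes it.
; While the Gate is open, E or the gamepad left face button sets PickedUpKey on the character, prints a confirmation and destroys the key.
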(event `Key|E`
  (params (Key :type "Key Structure"))
  ;[0.2263 0.2519 1] Si le joueur appuie sur E ou le bouton d'interraction de sa manette, on passe le bouléen pick up key à true ce qui veut dire qu'il peut ouvrir une porte. On détruit la clé après.
  ;;[0.2263 0.2519 1] Si le joueur appuie sur E ou sur le bouton X (ou carré ) d'une manette
  (:`Pressed`
    (`/Engine/EditorBlueprintResources/StandardMacros.Gate` true :!label _label
      (:`Exit`
        (set `/Game/StarWarsCore/Blueprints/Characters/BP_PlayerCharacter.Picked up key` true (stale `self.Box.OnComponentBeginOverlap` _asbp_player_character)) ; Dit au player qu'il possède une clé
        (`KismetSystemLibrary.PrintString` "La clé est  prise")
        (`self.K2_DestroyActor`) ; Detruit la clé
      ))))

(event `Key|Gamepad_FaceButton_Left`
  (params (Key :type "Key Structure"))
  ;[0.2263 0.2519 1] Si le joueur appuie sur E ou le bouton d'interraction de sa manette, on passe le bouléen pick up key à true ce qui veut dire qu'il peut ouvrir une porte. On détruit la clé après.
  ;;[0.2263 0.2519 1] Si le joueur appuie sur E ou sur le bouton X (ou carré ) d'une manette
  (:`Pressed`
    (goto _label)))

(event `self.Box.OnComponentBeginOverlap`
  (params (OverlappedComponent :type "PrimitiveComponent Object Reference") (OtherActor :type "Actor Object Reference") (OtherComp :type "PrimitiveComponent Object Reference") (OtherBodyIndex :type Integer) (bFromSweep :type Boolean) (SweepResult :type "HitResult Structure (by ref)"))
  ;[0.2263 0.2519 1] Si le joueur appuie sur E ou le bouton d'interraction de sa manette, on passe le bouléen pick up key à true ce qui veut dire qu'il peut ouvrir une porte. On détruit la clé après.
  (bind _asbp_player_character (cast `/Game/StarWarsCore/Blueprints/Characters/BP_PlayerCharacter` OtherActor))
  ;;[0.2263 0.2519 1] Affiche le message expliquant au joueur comment ramasser l'objet
  (bind _returnvalue (`|CreateWidget` "/Game/StarWarsCore/Blueprints/Actors/EnvironmentObject/Door/WB_PickUp.WB_PickUp_C" (`GameplayStatics.GetPlayerController` 0)))
  (bind _output_get (set `self.PickUp Widget` _returnvalue))
  (`UserWidget.AddToViewport` _output_get 0)
  (`self.EnableInput` (`GameplayStatics.GetPlayerController` 0))
  (goto _label :!via `Open`))

(event `self.Box.OnComponentEndOverlap`
  (params (OverlappedComponent :type "PrimitiveComponent Object Reference") (OtherActor :type "Actor Object Reference") (OtherComp :type "PrimitiveComponent Object Reference") (OtherBodyIndex :type Integer))
  ;[0.2263 0.2519 1] Si le joueur appuie sur E ou le bouton d'interraction de sa manette, on passe le bouléen pick up key à true ce qui veut dire qu'il peut ouvrir une porte. On détruit la clé après.
  (cast `/Game/StarWarsCore/Blueprints/Characters/BP_PlayerCharacter` OtherActor)
  ;;[0.2263 0.2519 1] Desactive le message disant au joueur comment ramasser l'objet
  (bind _pickup_widget (`self.PickUp Widget`)
    (:`then`
      (`Widget.RemoveFromParent` _pickup_widget)
      (`self.DisableInput` (`GameplayStatics.GetPlayerController` 0) null)
      (goto _label :!via `Close`))
    (:`else`)))

(fn `UserConstructionScript`)