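; Locked door actor that opens along Z when the player interacts while holding a key.
; Detection zone overlap shows a prompt widget, enables input and opens a gate for the E or gamepad interact press.
; With a key, a timeline adds a lerped offset to the current location each update, consumes the key and disables overlap events.
; Without one, a temporary "door closed" widget appears.
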(event `Key|E`
  (params (Key :type "Key Structure"))
  ;[0.2263 0.2519 1] Si le joueur a une clé (si la variable Picked up key dans le BP_PlayerCharacter est true) alors le joueur lance l'ouverture de la porte. Pick up key devient alors faux ( le joueur n'a plus de clé) et la zone de detection de la porte se desactive (le joueur ne peut plus interragir avec elle)
  ;;[0.284 0.4184 1] Si il appuie sur X (manette) ou sur E
  (:`Pressed`
    (if (`/Game/StarWarsCore/Blueprints/Characters/BP_PlayerCharacter.Picked up key` (stale `self.DetectionZone.OnComponentBeginOverlap` _asbp_player_character)) :!label _label
      (`/Engine/EditorBlueprintResources/StandardMacros.Gate` true :!label _label_2
        (:`Exit`
          ;;[0.2263 0.2519 1] Crée l'animation d'ouverture de la porte
          (bind (_direction _newtrack_0) (`Timeline|Timeline`)
            (:`Update`
              (`self.K2_SetActorLocation` (+ (`self.K2_GetActorLocation`) (`KismetMathLibrary.MakeVector` 0.0 0.0 (`KismetMathLibrary.Lerp` 0.0 (`self.Open Door`) _newtrack_0))))
              (set `/Game/StarWarsCore/Blueprints/Characters/BP_PlayerCharacter.Picked up key` false (stale `self.DetectionZone.OnComponentBeginOverlap` _asbp_player_character)) ; Rend la clé a usage unique
              (set `PrimitiveComponent.bGenerateOverlapEvents` false (`self.DetectionZone`)) ; Permet de ne plus pouvoir entrer en contact avec le trigger après utilisation
            ))))
      (else
        ;;[0.2263 0.2519 1] Indique au joueur grâce à un Widget que la porte est fermée et qu'il lui faut une clé
        (`KismetSystemLibrary.PrintString` "Door is locked")
        (bind _returnvalue (`|CreateWidget` "/Game/StarWarsCore/Blueprints/Actors/EnvironmentObject/Door/WB_DoorIsClosed.WB_DoorIsClosed_C" (`GameplayStatics.GetPlayerController` 0)))
        (bind _output_get (set `self.DoorCloseWidget` _returnvalue))
        (`UserWidget.AddToViewport` _output_get 0)
        (`KismetSystemLibrary.Delay` (`self.WidgetDuration`))
        (`Widget.RemoveFromParent` (`self.DoorCloseWidget`)) ; Enleve definitivement le widget
        (set `self.DoorCloseWidget` null)))))

(event `Key|Gamepad_FaceButton_Left`
  (params (Key :type "Key Structure"))
  ;[0.2263 0.2519 1] Si le joueur a une clé (si la variable Picked up key dans le BP_PlayerCharacter est true) alors le joueur lance l'ouverture de la porte. Pick up key devient alors faux ( le joueur n'a plus de clé) et la zone de detection de la porte se desactive (le joueur ne peut plus interragir avec elle)
  ;;[0.284 0.4184 1] Si il appuie sur X (manette) ou sur E
  (:`Pressed`
    (goto _label)))

(event `self.DetectionZone.OnComponentBeginOverlap`
  (params (OverlappedComponent :type "PrimitiveComponent Object Reference") (OtherActor :type "Actor Object Reference") (OtherComp :type "PrimitiveComponent Object Reference") (OtherBodyIndex :type Integer) (bFromSweep :type Boolean) (SweepResult :type "HitResult Structure (by ref)"))
  (bind _returnvalue (`GameplayStatics.GetPlayerController` 0))
  ;[0.2263 0.2519 1] Si le joueur a une clé (si la variable Picked up key dans le BP_PlayerCharacter est true) alors le joueur lance l'ouverture de la porte. Pick up key devient alors faux ( le joueur n'a plus de clé) et la zone de detection de la porte se desactive (le joueur ne peut plus interragir avec elle)
  (bind _asbp_player_character (cast `/Game/StarWarsCore/Blueprints/Characters/BP_PlayerCharacter` OtherActor))
  ;;[0.2263 0.2519 1] Affiche le message expliquant comment utiliser la porte
  (bind _returnvalue_2 (`|CreateWidget` "/Game/StarWarsCore/Blueprints/Actors/EnvironmentObject/Door/WB_InteractWithDoor.WB_InteractWithDoor_C" _returnvalue))
  (bind _output_get (set `self.WidgetInteractWithDoor` _returnvalue_2))
  (`UserWidget.AddToViewport` _output_get 0)
  (`self.EnableInput` _returnvalue)
  (goto _label_2 :!via `Open`))

(event `self.DetectionZone.OnComponentEndOverlap`
  (params (OverlappedComponent :type "PrimitiveComponent Object Reference") (OtherActor :type "Actor Object Reference") (OtherComp :type "PrimitiveComponent Object Reference") (OtherBodyIndex :type Integer))
  ;[0.2263 0.2519 1] Si le joueur a une clé (si la variable Picked up key dans le BP_PlayerCharacter est true) alors le joueur lance l'ouverture de la porte. Pick up key devient alors faux ( le joueur n'a plus de clé) et la zone de detection de la porte se desactive (le joueur ne peut plus interragir avec elle)
  (cast `/Game/StarWarsCore/Blueprints/Characters/BP_PlayerCharacter` OtherActor)
  ;;[0.2263 0.2519 1] Desactive le message expliquant comment utiliser la porte
  (bind _widgetinteractwithdoor (`self.WidgetInteractWithDoor`)
    (:`then`
      (`Widget.RemoveFromParent` _widgetinteractwithdoor)
      (`self.DisableInput` (`GameplayStatics.GetPlayerController` 0))
      (goto _label_2 :!via `Close`))
    (:`else`)))

(fn `UserConstructionScript`)