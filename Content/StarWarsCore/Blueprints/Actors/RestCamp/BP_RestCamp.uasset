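; Rest camp actor that lets the player rest while inside its box and registers itself as the player's last used camp.
; On BeginPlay, StockIA snapshots the class, location, SData and reference of every BP_Base_NPC in the level.
; RespawnIA destroys those tracked NPCs and respawns them from the snapshot, but nothing in this Blueprint's live graph calls it.
; ScaleLevel is an unfinished stub with disconnected logic.
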(event `self.ReceiveBeginPlay`
  (`self.StockIA`))

(event `self.Box.OnComponentBeginOverlap`
  (params (OverlappedComponent :type "PrimitiveComponent Object Reference") (OtherActor :type "Actor Object Reference") (OtherComp :type "PrimitiveComponent Object Reference") (OtherBodyIndex :type Integer) (bFromSweep :type Boolean) (SweepResult :type "HitResult Structure (by ref)"))
  (bind _asbp_player_character (cast `/Game/StarWarsCore/Blueprints/Characters/BP_PlayerCharacter` OtherActor))
  (set `/Game/StarWarsCore/Blueprints/Characters/BP_PlayerCharacter.CanRest` true _asbp_player_character)
  (set `/Game/StarWarsCore/Blueprints/Characters/BP_PlayerCharacter.LastRestCampUse` self _asbp_player_character))

(event `self.Box.OnComponentEndOverlap`
  (params (OverlappedComponent :type "PrimitiveComponent Object Reference") (OtherActor :type "Actor Object Reference") (OtherComp :type "PrimitiveComponent Object Reference") (OtherBodyIndex :type Integer))
  (bind _asbp_player_character (cast `/Game/StarWarsCore/Blueprints/Characters/BP_PlayerCharacter` OtherActor))
  (set `/Game/StarWarsCore/Blueprints/Characters/BP_PlayerCharacter.CanRest` false _asbp_player_character))

(fn `RespawnIA`
  (for _array_element (`self.ActorRef`)
    (`/Engine/EditorBlueprintResources/StandardMacros.IsValid` _array_element
      (:`Is Valid`
        (`self.K2_DestroyActor` _array_element))))
  (`KismetArrayLibrary.Array_Clear` (`self.ActorRef`))
  (for (_ _array_index) (`self.ClassRef`)
    (bind _returnvalue (`|SpawnActorFromClass` (`|GetArrayItem` (`self.ClassRef`) _array_index) (`KismetMathLibrary.MakeTransform` (`|GetArrayItem` (`self.PositionAI`) _array_index)) "Undefined" "MultiplyWithRoot" null (`|GetArrayItem` (`self.S_DataAI`) _array_index) null))
    (`KismetArrayLibrary.Array_Add` (`self.ActorRef`) _returnvalue)))

(fn `ScaleLevel`
  (locals (Index :type Integer)))

(fn `StockIA`
  (`BlueprintMapLibrary.Map_Clear` (`self.ClassAndPosition`))
  (bind _outactors (`GameplayStatics.GetAllActorsOfClass` "/Game/StarWarsCore/Blueprints/Characters/NPC/BP_Base_NPC.BP_Base_NPC_C"))
  (for _array_element _outactors
    (`KismetArrayLibrary.Array_Add` (`self.ClassRef`) (`GameplayStatics.GetObjectClass` _array_element))
    (`KismetArrayLibrary.Array_Add` (`self.PositionAI`) (`self.K2_GetActorLocation` _array_element))
    (`KismetArrayLibrary.Array_Add` (`self.ActorRef`) _array_element)
    (`KismetArrayLibrary.Array_Add` (`self.S_DataAI`) (`/Game/StarWarsCore/Blueprints/Characters/NPC/BP_Base_NPC.S_Data` _array_element))))

(fn `UserConstructionScript`)