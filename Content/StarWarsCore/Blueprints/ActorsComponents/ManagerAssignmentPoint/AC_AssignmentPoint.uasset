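; Actor component that lets the player spend assignment points on Strength, Vitality, Armor or Stamina and toggles the assignment menu.
; Each spend increments that stat's point count, pushes points times a coefficient to AC_Stats, then subtracts an available point.
; Only Strength and Armor add the cached base value here.
; Reset sets available points to player level and restores cached stats; opening the menu deactivates character movement.
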(event `ChangeOnePointOnDesireStat`
  (params (Selection :type "/Game/StarWarsCore/Blueprints/ActorsComponents/ManagerAssignmentPoint/Data/E_AssignmentPoints Enum" :default "NewEnumerator0"))
  ;[1 0.75 0] Main Event
  (`self.ChangeOnePointOnStat` Selection))

(event `ModifyPointToArmor`
  (params (Add :type Boolean))
  ;[1 0 0.7833] Modify Point
  (`self.ModifyPointToStatArmor` Add))

(event `ModifyPointToVitality`
  (params (Add :type Boolean))
  ;[1 0 0.7833] Modify Point
  (`self.ModifyPointToStatVitality` Add))

(event `ModifyPointToStamina`
  (params (Add :type Boolean))
  ;[1 0 0.7833] Modify Point
  (`self.ModifyPointToStatStamina` Add))

(event `ModifyPointToStrength`
  (params (Add :type Boolean))
  ;[1 0 0.7833] Modify Point
  (`self.ModifyPointToStatStrength` Add))

(event `ResetAssignmentPoint`
  ;[1 0 0.7833] Modify Point
  (`self.ResetAssignmentPoints`))

(fn `ChangeOnePointOnStat`
  (params (Selection :type "/Game/StarWarsCore/Blueprints/ActorsComponents/ManagerAssignmentPoint/Data/E_AssignmentPoints Enum" :default "NewEnumerator0"))
  (bind (_strengthpoints _armorpoints _vitalitypoints _staminapoints) (break `/Game/StarWarsCore/Blueprints/ActorsComponents/ManagerAssignmentPoint/Data/S_AssignmentPointData` (`self.S_AssignmentPointsData`)))
  (switch `/Game/StarWarsCore/Blueprints/ActorsComponents/ManagerAssignmentPoint/Data/E_AssignmentPoints` Selection
    (:`NewEnumerator0`
      (`/Engine/EditorBlueprintResources/StandardMacros.IncrementInt` _strengthpoints
        (:`  `
          (`self.ModifyPointToStrength` true))))
    (:`NewEnumerator1`
      (`/Engine/EditorBlueprintResources/StandardMacros.IncrementInt` _vitalitypoints
        (:`  `
          (`self.ModifyPointToVitality` true))))
    (:`NewEnumerator2`
      (`/Engine/EditorBlueprintResources/StandardMacros.IncrementInt` _armorpoints
        (:`  `
          (`self.ModifyPointToArmor` true))))
    (:`NewEnumerator3`
      (`/Engine/EditorBlueprintResources/StandardMacros.IncrementInt` _staminapoints
        (:`  `
          (`self.ModifyPointToStamina` true)))))
  (`/Game/StarWarsCore/Blueprints/ActorsComponents/ManagerStats/AC_Stats.SubstractAssignmentPoints` (`Actor.GetComponentByClass` (`GameplayStatics.GetPlayerCharacter` 0) "/Game/StarWarsCore/Blueprints/ActorsComponents/ManagerStats/AC_Stats.AC_Stats_C")))

(fn `CheckIfHavePoints`
  (returns (HavePoints :type Boolean))
  (return (> (`.AssignmentPoint_35_B60287BC4327B0C008322785D9F0AFA8` (break `/Game/StarWarsCore/Blueprints/ActorsComponents/ManagerStats/Data/S_Stats` (`/Game/StarWarsCore/Blueprints/ActorsComponents/ManagerStats/AC_Stats.S_Stats` (`Actor.GetComponentByClass` (`GameplayStatics.GetPlayerCharacter` 0) "/Game/StarWarsCore/Blueprints/ActorsComponents/ManagerStats/AC_Stats.AC_Stats_C")))) 0.0)))

(fn `ModifyPointToStatArmor`
  (params (Add :type Boolean))
  (bind _returnvalue (`Actor.GetComponentByClass` (`GameplayStatics.GetPlayerCharacter` 0) "/Game/StarWarsCore/Blueprints/ActorsComponents/ManagerStats/AC_Stats.AC_Stats_C"))
  (message `/Game/StarWarsCore/Blueprints/ActorsComponents/ManagerStats/BPI_Stats.SetAmor` _returnvalue (+ (* (`.ArmorPoints_5_75D6FEDA46E36EA81B9668921797D3D9` (break `/Game/StarWarsCore/Blueprints/ActorsComponents/ManagerAssignmentPoint/Data/S_AssignmentPointData` (`self.S_AssignmentPointsData`))) (`self.ArmorPointCoefficient`)) (`.Armor_25_68B2E5B948B13B9A2B9B20BB09FFB5E6` (break `/Game/StarWarsCore/Blueprints/ActorsComponents/ManagerStats/Data/S_Stats` (`/Game/StarWarsCore/Blueprints/ActorsComponents/ManagerStats/AC_Stats.S Stats Cache` _returnvalue))))))

(fn `ModifyPointToStatStamina`
  (params (Add :type Boolean))
  (message `/Game/StarWarsCore/Blueprints/ActorsComponents/ManagerStats/BPI_Stats.SetMaxStamina` (`Actor.GetComponentByClass` (`GameplayStatics.GetPlayerCharacter` 0) "/Game/StarWarsCore/Blueprints/ActorsComponents/ManagerStats/AC_Stats.AC_Stats_C") (* (`.StaminaPoints_9_B0D4FAB4435DF3EAA15E81A675FA821C` (break `/Game/StarWarsCore/Blueprints/ActorsComponents/ManagerAssignmentPoint/Data/S_AssignmentPointData` (`self.S_AssignmentPointsData`))) (`self.StaminaPointCoefficient`))))

(fn `ModifyPointToStatStrength`
  (params (Add :type Boolean))
  (bind _returnvalue (`Actor.GetComponentByClass` (`GameplayStatics.GetPlayerCharacter` 0) "/Game/StarWarsCore/Blueprints/ActorsComponents/ManagerStats/AC_Stats.AC_Stats_C"))
  (message `/Game/StarWarsCore/Blueprints/ActorsComponents/ManagerStats/BPI_Stats.SetStrength` _returnvalue (+ (* (`.StrengthPoints_3_EB20B95C4EFF6E0E8FFED8B1F4624F40` (break `/Game/StarWarsCore/Blueprints/ActorsComponents/ManagerAssignmentPoint/Data/S_AssignmentPointData` (`self.S_AssignmentPointsData`))) (`self.StrengthPointCoefficient`)) (`.Strength_20_0D938E1D481D25F6A224C6AE5C7A2D49` (break `/Game/StarWarsCore/Blueprints/ActorsComponents/ManagerStats/Data/S_Stats` (`/Game/StarWarsCore/Blueprints/ActorsComponents/ManagerStats/AC_Stats.S Stats Cache` _returnvalue))))))

(fn `ModifyPointToStatVitality`
  (params (Add :type Boolean))
  (message `/Game/StarWarsCore/Blueprints/ActorsComponents/ManagerStats/BPI_Stats.SetVitality` (`Actor.GetComponentByClass` (`GameplayStatics.GetPlayerCharacter` 0) "/Game/StarWarsCore/Blueprints/ActorsComponents/ManagerStats/AC_Stats.AC_Stats_C") (* (`.VitalityPoints_7_E9A923E44D3E359A745E2AB7A5DEBBDB` (break `/Game/StarWarsCore/Blueprints/ActorsComponents/ManagerAssignmentPoint/Data/S_AssignmentPointData` (`self.S_AssignmentPointsData`))) (`self.VitalityPointCoefficient`))))

(fn `ResetAssignmentPoints`
  (bind _returnvalue (`Actor.GetComponentByClass` (`GameplayStatics.GetPlayerCharacter` 0) "/Game/StarWarsCore/Blueprints/ActorsComponents/ManagerStats/AC_Stats.AC_Stats_C"))
  (bind _s_stats (`/Game/StarWarsCore/Blueprints/ActorsComponents/ManagerStats/AC_Stats.S_Stats` _returnvalue))
  (bind ((`Strength_20_0D938E1D481D25F6A224C6AE5C7A2D49` _strength) (`Armor_25_68B2E5B948B13B9A2B9B20BB09FFB5E6` _armor) (`Vitality_28_97E612684821BF45F3641790379A02EB` _vitality) (`MaxStamina_32_76CEAF3A452EF80B0388CDA4568F5E45` _maxstamina)) (break `/Game/StarWarsCore/Blueprints/ActorsComponents/ManagerStats/Data/S_Stats` (`/Game/StarWarsCore/Blueprints/ActorsComponents/ManagerStats/AC_Stats.S Stats Cache` _returnvalue)))
  (setmembers `/Game/StarWarsCore/Blueprints/ActorsComponents/ManagerStats/Data/S_Stats` :`StructRef` _s_stats :`AssignmentPoint` (`KismetMathLibrary.Conv_IntToDouble` (`.Level_14_AC96BB6B44E2483A794787BE8E04C43B` (break `/Game/StarWarsCore/Blueprints/ActorsComponents/ManagerStats/Data/S_Stats` _s_stats))))
  (setmembers `/Game/StarWarsCore/Blueprints/ActorsComponents/ManagerAssignmentPoint/Data/S_AssignmentPointData` :`StructRef` (`self.S_AssignmentPointsData`) :`StrengthPoints` 0 :`ArmorPoints` 0 :`VitalityPoints` 0 :`StaminaPoints` 0)
  (setmembers `/Game/StarWarsCore/Blueprints/ActorsComponents/ManagerStats/Data/S_Stats` :`StructRef` (`/Game/StarWarsCore/Blueprints/ActorsComponents/ManagerStats/AC_Stats.S_Stats` (`Actor.GetComponentByClass` (`GameplayStatics.GetPlayerCharacter` 0) "/Game/StarWarsCore/Blueprints/ActorsComponents/ManagerStats/AC_Stats.AC_Stats_C")) :`Strength` _strength :`Armor` _armor :`Vitality` _vitality :`MaxStamina` _maxstamina))

(fn `ShowAssignmentMenu`
  (bind _charactermovement (`Character.CharacterMovement` (`GameplayStatics.GetPlayerCharacter` 0)))
  (bind _wb_assignmentpoint (`self.WB_AssignmentPoint`)
    (:`then`
      (`CommonActivatableWidget.DeactivateWidget` _wb_assignmentpoint)
      (`Widget.RemoveFromParent` _wb_assignmentpoint)
      (set `self.WB_AssignmentPoint` null)
      (`WidgetBlueprintLibrary.SetInputMode_GameOnly` (`GameplayStatics.GetPlayerController` 0) true)
      ;[0.2263 0.2519 1] Active et desactive le mouvement du joueur quand  il est dans le menu d'assignation
      (`self.Activate` _charactermovement false))
    (:`else`
      (bind _returnvalue (`|CreateWidget` "/Game/StarWarsCore/Blueprints/ActorsComponents/ManagerAssignmentPoint/Widget/WB_AssignmentPoint.WB_AssignmentPoint_C"))
      (bind _output_get (set `self.WB_AssignmentPoint` _returnvalue))
      (`UserWidget.AddToViewport` _output_get 0)
      (`self.Deactivate` _charactermovement))))