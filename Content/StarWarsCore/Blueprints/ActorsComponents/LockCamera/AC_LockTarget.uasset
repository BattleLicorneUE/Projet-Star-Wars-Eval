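; AC_LockTarget is a lock-on camera component that keeps the first player's view turned toward a nearby NPC.
; On BeginPlay, ChooseTarget maps BP_Base_NPC actors with non-negative health within a short range by player distance, then stores and debug-prints the closest.
; Each Tick, while locked, it overrides only the controller's yaw with a look-at rotation toward that target, preserving pitch and roll.
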(event `self.ReceiveBeginPlay`
  (`self.ChooseTarget`))

(event `self.ReceiveTick`
  (params (DeltaSeconds :type "Float (single-precision)"))
  (if (`self.Target`)
    (`self.LockCameraToTarget`)))

(fn `ChooseTarget`
  (set `self.Target` true)
  (`BlueprintMapLibrary.Map_Clear` (`self.DistanceToPlayer`))
  (bind _outactors (`GameplayStatics.GetAllActorsOfClass` "/Game/StarWarsCore/Blueprints/Characters/NPC/BP_Base_NPC.BP_Base_NPC_C"))
  (for _array_element _outactors
    (if (>= (`.Health_6_941275B54471A39A9377D7B954810D24` (break `/Game/StarWarsCore/IA/Data/S_DataAI` (`/Game/StarWarsCore/Blueprints/Characters/NPC/BP_Base_NPC.S_Data` _array_element))) 0.0)
      (bind _returnvalue (`Actor.GetDistanceTo` _array_element (`GameplayStatics.GetPlayerCharacter` 0)))
      (if (<= _returnvalue 600.0)
        (`BlueprintMapLibrary.Map_Add` (`self.DistanceToPlayer`) _returnvalue _array_element))))
  (bind _keys (`BlueprintMapLibrary.Map_Keys` (`self.DistanceToPlayer`)))
  (bind _values (`BlueprintMapLibrary.Map_Values` (`self.DistanceToPlayer`)))
  (bind _output (`|GetArrayItem` _values (`KismetMathLibrary.MinOfFloatArray` _keys)))
  (`KismetSystemLibrary.PrintString` (`KismetSystemLibrary.GetDisplayName` _output))
  (set `self.TargetToLock` _output))

(fn `LockCameraToTarget`
  (bind _returnvalue (`GameplayStatics.GetPlayerController` 0))
  (bind (_returnvalue_roll _returnvalue_pitch) (`KismetMathLibrary.BreakRotator` (`Controller.GetControlRotation` _returnvalue)))
  (bind (_returnvalue_roll_2 _returnvalue_pitch_2 _returnvalue_yaw) (`KismetMathLibrary.BreakRotator` (`KismetMathLibrary.FindLookAtRotation` (`Actor.K2_GetActorLocation` (`GameplayStatics.GetPlayerCharacter` 0)) (`Actor.K2_GetActorLocation` (`self.TargetToLock`)))))
  (`/Engine/EditorBlueprintResources/StandardMacros.IsValid` (`self.TargetToLock`)
    (:`Is Valid`
      (`Controller.SetControlRotation` _returnvalue (`KismetMathLibrary.MakeRotator` _returnvalue_roll _returnvalue_pitch _returnvalue_yaw)))))