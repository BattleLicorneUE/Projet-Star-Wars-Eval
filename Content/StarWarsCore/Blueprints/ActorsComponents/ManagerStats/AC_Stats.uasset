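; Actor component holding RPG stats (HP, XP, level, stamina, strength, damage, armor, vitality, assignment points) in one SStats struct.
; Set and Modify events route to helpers, mostly clamped; vitality adds to max HP, and SetMaxPv rescales current HP proportionally.
; Filling XP or changing level calls the player character's AC_ManagerExperience.
; It also provides strength-scaled damage and armor-percentage reduction, plus debug level-up and print keys.
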(event `Key|L`
  (params (Key :type "Key Structure"))
  ;[0.1738 0 1] DebugKey
  (:`Pressed`
    (`/Game/StarWarsCore/Blueprints/ActorsComponents/ManagerExperience/AC_ManagerExperience.LevelUp` (`Actor.GetComponentByClass` (`GameplayStatics.GetPlayerCharacter` 0) "/Game/StarWarsCore/Blueprints/ActorsComponents/ManagerExperience/AC_ManagerExperience.AC_ManagerExperience_C"))))

(event `Key|B`
  (params (Key :type "Key Structure"))
  ;[0.1738 0 1] DebugKey
  (:`Pressed`
    (`self.PrintAllStats`)))

(event `self.ReceiveBeginPlay`
  ;[1 0.1667 0.1667] Begin Play
  (`/Game/StarWarsCore/Blueprints/ActorsComponents/ManagerStats/BPI_Stats.ApplyVitality`)
  (`self.InitCurrentPv`)
  (`self.InitStamina`))

(event `/Game/StarWarsCore/Blueprints/ActorsComponents/ManagerStats/BPI_Stats.ModifyCurrentPv`
  (params (Amount :type "Float (double-precision)") (Add :type Boolean))
  ;[0 1 0.2245] PV Modifier
  (`self.CurrentPvModifier` Amount Add))

(event `/Game/StarWarsCore/Blueprints/ActorsComponents/ManagerStats/BPI_Stats.XpNeedSet`
  (params (Amount :type "Float (double-precision)"))
  ;[0.1332 0.5271 1] XP Modifier and Level
  (`self.SetXpNeed` Amount))

(event `/Game/StarWarsCore/Blueprints/ActorsComponents/ManagerStats/BPI_Stats.ModifyCurrentXp`
  (params (Amount :type "Float (double-precision)") (Add :type Boolean))
  ;[0.1332 0.5271 1] XP Modifier and Level
  (`self.CurrentXpModifier` Amount Add)
  (`self.CheckIfLevelUp`))

(event `/Game/StarWarsCore/Blueprints/ActorsComponents/ManagerStats/BPI_Stats.ModifyMaxPv`
  (params (Amount :type "Float (double-precision)") (Add :type Boolean))
  ;[0 1 0.2245] PV Modifier
  (`self.MaxPvModifier` Amount Add))

(event `/Game/StarWarsCore/Blueprints/ActorsComponents/ManagerStats/BPI_Stats.ResetCurrentXp`
  ;[0.1332 0.5271 1] XP Modifier and Level
  (`self.CurrentXpReset`))

(event `/Game/StarWarsCore/Blueprints/ActorsComponents/ManagerStats/BPI_Stats.SetMaxPv`
  (params (Amount :type "Float (double-precision)"))
  ;[0 1 0.2245] PV Modifier
  (bind _oldmaxpv (`self.SaveMaxPv`))
  (`self.MaxPvSet` Amount _oldmaxpv))

(event `/Game/StarWarsCore/Blueprints/ActorsComponents/ManagerStats/BPI_Stats.ModifyLevel`
  (params (Amount :type Integer) (Add :type Boolean))
  ;[0.1332 0.5271 1] XP Modifier and Level
  (`self.LevelModifier` Amount Add)
  (`self.InitXpAndPvInTermOfLevel`))

(event `/Game/StarWarsCore/Blueprints/ActorsComponents/ManagerStats/BPI_Stats.ModifyStrength`
  (params (Amount :type "Float (double-precision)") (Add :type Boolean))
  ;[1 0 0] Strength Modifier
  (`self.StrengthModifier` Amount Add))

(event `/Game/StarWarsCore/Blueprints/ActorsComponents/ManagerStats/BPI_Stats.ModifyBaseDamage`
  (params (Amount :type "Float (double-precision)") (Add :type Boolean))
  ;[1 0.4095 0] Damage Modifier
  (`self.BaseDamageModifier` Amount Add))

(event `/Game/StarWarsCore/Blueprints/ActorsComponents/ManagerStats/BPI_Stats.SetMaxStamina`
  (params (Amount :type "Float (double-precision)"))
  ;[0.4645 1 0.1094] Stamina Modifier
  (`self.MaxStaminaSet` Amount))

(event `/Game/StarWarsCore/Blueprints/ActorsComponents/ManagerStats/BPI_Stats.SetStrength`
  (params (Amount :type "Float (double-precision)"))
  ;[1 0 0] Strength Modifier
  (`self.StrengthSet` Amount))

(event `/Game/StarWarsCore/Blueprints/ActorsComponents/ManagerStats/BPI_Stats.ModifyMaxStamina`
  (params (Amount :type "Float (double-precision)") (Add :type Boolean))
  ;[0.4645 1 0.1094] Stamina Modifier
  (`self.MaxStaminaModifier` Amount Add))

(event `/Game/StarWarsCore/Blueprints/ActorsComponents/ManagerStats/BPI_Stats.SetBaseDamage`
  (params (Amount :type "Float (double-precision)"))
  ;[1 0.4095 0] Damage Modifier
  (`self.BaseDamageSet` Amount))

(event `/Game/StarWarsCore/Blueprints/ActorsComponents/ManagerStats/BPI_Stats.ModifyCurrentStamina`
  (params (Amount :type "Float (double-precision)") (Add :type Boolean))
  ;[0.4645 1 0.1094] Stamina Modifier
  (`self.CurrentStaminaModifier` Amount Add))

(event `/Game/StarWarsCore/Blueprints/ActorsComponents/ManagerStats/BPI_Stats.SetAmor`
  (params (Amount :type "Float (double-precision)"))
  ;[1 0.9568 0.1188] Armor Modifier
  (`self.ArmorSet` Amount))

(event `/Game/StarWarsCore/Blueprints/ActorsComponents/ManagerStats/BPI_Stats.SetVitality`
  (params (Amount :type "Float (double-precision)"))
  ;[0 1 0.8243] Vitality Modifier
  (`self.VitalitySet` Amount))

(event `/Game/StarWarsCore/Blueprints/ActorsComponents/ManagerStats/BPI_Stats.ModifyArmor`
  (params (Amount :type "Float (double-precision)") (Add :type Boolean))
  ;[1 0.9568 0.1188] Armor Modifier
  (`self.ArmorModifier` Amount Add))

(event `/Game/StarWarsCore/Blueprints/ActorsComponents/ManagerStats/BPI_Stats.ModifyVitality`
  (params (Amount :type "Float (double-precision)") (Add :type Boolean))
  ;[0 1 0.8243] Vitality Modifier
  (`self.VitalityModifier` Amount Add))

(event `/Game/StarWarsCore/Blueprints/ActorsComponents/ManagerStats/BPI_Stats.ModifyAssignmentPoint`
  (params (Amount :type "Float (double-precision)") (Add :type Boolean))
  ;[0.182 0 1] Modify AssignmentPoint
  (`self.AssignmentPointModifier` Amount Add))

(event `/Game/StarWarsCore/Blueprints/ActorsComponents/ManagerStats/BPI_Stats.ApplyVitality`
  ;[0 1 0.8243] Vitality Modifier
  (`self.VitalityApply`))

(fn `ApplyArmorReduction`
  (params (Damage :type "Float (double-precision)"))
  (returns (DamageWithReduction :type "Float (double-precision)"))
  (bind _damagewithreduction (`self.CalculateArmorReduction` Damage))
  (return _damagewithreduction))

(fn `ApplyDamageWithForce`
  (returns (Damage :type "Float (double-precision)"))
  (bind ((`Strength_20_0D938E1D481D25F6A224C6AE5C7A2D49` _strength) (`BaseDamage_23_3584FFBF4B586CEA3D9B56BAA9D3A34F` _basedamage)) (break `/Game/StarWarsCore/Blueprints/ActorsComponents/ManagerStats/Data/S_Stats` (`self.S_Stats`)))
  (return (+ (* _strength (`self.StrengthCoefficient`)) _basedamage)))

(fn `ArmorModifier`
  (params (Amount :type "Float (double-precision)") (Add :type Boolean))
  (if Add
    (`self.AddArmor`)
    (else
      (`self.SubstractArmor`))))

(fn `ArmorSet`
  (params (Amount :type "Float (double-precision)"))
  (setmembers `/Game/StarWarsCore/Blueprints/ActorsComponents/ManagerStats/Data/S_Stats` :`StructRef` (`self.S_Stats`) :`Armor` (`KismetMathLibrary.FClamp` Amount)))

(fn `AssignmentPointModifier`
  (params (Amount :type "Float (double-precision)") (Add :type Boolean))
  (bind ((`MaxLevel_16_D89379EE46214A511074F2947D840039` _maxlevel) (`AssignmentPoint_35_B60287BC4327B0C008322785D9F0AFA8` _assignmentpoint)) (break `/Game/StarWarsCore/Blueprints/ActorsComponents/ManagerStats/Data/S_Stats` (`self.S_Stats`)))
  (if (== _assignmentpoint _maxlevel)
    _
    (elif Add
      (`self.AddToAssignmentPoint`)
      (else
        (`self.SubstractAssignmentPoint`)))))

(fn `BaseDamageModifier`
  (params (Amount :type "Float (double-precision)") (Add :type Boolean))
  (if Add
    (`self.AddToDamage` Amount)
    (else
      (`self.SubStractToDamage` Amount))))

(fn `BaseDamageSet`
  (params (Amount :type "Float (double-precision)"))
  (setmembers `/Game/StarWarsCore/Blueprints/ActorsComponents/ManagerStats/Data/S_Stats` :`StructRef` (`self.S_Stats`) :`BaseDamage` (`KismetMathLibrary.FClamp` Amount 0.0 999999.0)))

(fn `CalculateArmorReduction`
  (params (Damage :type "Float (double-precision)"))
  (returns (DamageWithReduction :type "Float (double-precision)"))
  (return (- Damage (* (`.Armor_25_68B2E5B948B13B9A2B9B20BB09FFB5E6` (break `/Game/StarWarsCore/Blueprints/ActorsComponents/ManagerStats/Data/S_Stats` (`self.S_Stats`))) Damage))))

(fn `CheckIfLevelUp`
  (bind ((`CurrentXp_10_51121D1F442D30C6D07C1489015B0EAA` _currentxp) (`XpNeed_11_CCB70007410A7381AAED7DA2843A773C` _xpneed)) (break `/Game/StarWarsCore/Blueprints/ActorsComponents/ManagerStats/Data/S_Stats` (`self.S_Stats`)))
  (if (>= _currentxp _xpneed)
    (`/Game/StarWarsCore/Blueprints/ActorsComponents/ManagerExperience/AC_ManagerExperience.LevelUp` (`Actor.GetComponentByClass` (`GameplayStatics.GetPlayerCharacter` 0) "/Game/StarWarsCore/Blueprints/ActorsComponents/ManagerExperience/AC_ManagerExperience.AC_ManagerExperience_C"))
    (`self.CurrentXpReset`)))

(fn `CurrentPvModifier`
  (params (Amount :type "Float (double-precision)") (Add :type Boolean))
  (bind _amount (`local.Amount`))
  (if Add
    (`self.AddToCurrentPv` _amount)
    (else
      (`self.SubstractToCurrentPv` _amount))))

(fn `CurrentStaminaModifier`
  (params (Amount :type "Float (double-precision)") (Add :type Boolean))
  (if Add
    (`self.AddStamina`)
    (else
      (`self.SubstractStamina`))))

(fn `CurrentXpModifier`
  (params (Amount :type "Float (double-precision)") (Add :type Boolean))
  (bind _amount (`local.Amount`))
  (if Add
    (`self.AddToCurrentXp` _amount)
    (else
      (`self.SubstractToCurrentXp` _amount))))

(fn `CurrentXpReset`
  (setmembers `/Game/StarWarsCore/Blueprints/ActorsComponents/ManagerStats/Data/S_Stats` :`StructRef` (`self.S_Stats`) :`CurrentXp` 0.0))

(fn `InitCurrentPv`
  (bind _s_stats (`self.S_Stats`))
  (setmembers `/Game/StarWarsCore/Blueprints/ActorsComponents/ManagerStats/Data/S_Stats` :`StructRef` _s_stats :`CurrentPv` (`.MaxPv_7_C8AB5A71489D35F3081461989E3096F6` (break `/Game/StarWarsCore/Blueprints/ActorsComponents/ManagerStats/Data/S_Stats` _s_stats))))

(fn `InitStamina`
  (bind _s_stats (`self.S_Stats`))
  (setmembers `/Game/StarWarsCore/Blueprints/ActorsComponents/ManagerStats/Data/S_Stats` :`StructRef` _s_stats :`CurrentStamina` (`.MaxStamina_32_76CEAF3A452EF80B0388CDA4568F5E45` (break `/Game/StarWarsCore/Blueprints/ActorsComponents/ManagerStats/Data/S_Stats` _s_stats))))

(fn `InitXpAndPvInTermOfLevel`
  (`/Game/StarWarsCore/Blueprints/ActorsComponents/ManagerExperience/AC_ManagerExperience.ChangePvAndXpInTermsOfLevel` (`Actor.GetComponentByClass` (`GameplayStatics.GetPlayerCharacter` 0) "/Game/StarWarsCore/Blueprints/ActorsComponents/ManagerExperience/AC_ManagerExperience.AC_ManagerExperience_C")))

(fn `LevelModifier`
  (params (Amount :type Integer) (Add :type Boolean))
  (bind _amount (`local.Amount`))
  (if Add
    (`self.AddToLevel` _amount)
    (else
      (`self.SubstractToLevel` _amount))))

(fn `MaxPvModifier`
  (params (Amount :type "Float (double-precision)") (Add :type Boolean))
  (bind _amount (`local.Amount`))
  (if Add
    (`self.AddToMaxPv` _amount)
    (else
      (`self.SubstractToMaxPv` _amount))))

(fn `MaxPvSet`
  (params (Amount :type "Float (double-precision)") (OldMaxPv :type "Float (double-precision)"))
  (bind _s_stats (`self.S_Stats`))
  (setmembers `/Game/StarWarsCore/Blueprints/ActorsComponents/ManagerStats/Data/S_Stats` :`StructRef` _s_stats :`MaxPv` (`KismetMathLibrary.FClamp` Amount 0.0 999999999.0))
  (`/Game/StarWarsCore/Blueprints/ActorsComponents/ManagerStats/BPI_Stats.ApplyVitality`)
  (`self.SetCurrentPvInTermOfPourcentage` (`.CurrentPv_5_1DA056134E65C0C87CE3AAA131A0CB2C` (break `/Game/StarWarsCore/Blueprints/ActorsComponents/ManagerStats/Data/S_Stats` _s_stats)) (`local.OldMaxPv`)))

(fn `MaxStaminaModifier`
  (params (Amount :type "Float (double-precision)") (Add :type Boolean))
  (if Add
    (`self.AddToMaxStamina`)
    (else
      (`self.SubstractToMaxStamina`))))

(fn `MaxStaminaSet`
  (params (Amount :type "Float (double-precision)"))
  (setmembers `/Game/StarWarsCore/Blueprints/ActorsComponents/ManagerStats/Data/S_Stats` :`StructRef` (`self.S_Stats`) :`MaxStamina` (`KismetMathLibrary.FClamp` Amount 0.0 99999999.0)))

(fn `PrintAllStats`
  (bind (_currentpv _maxpv _currentxp _xpneed _level _maxlevel _strength _basedamage _armor _vitality _currentstamina _maxstamina _assignmentpoint) (break `/Game/StarWarsCore/Blueprints/ActorsComponents/ManagerStats/Data/S_Stats` (`self.S_Stats`)))
  (`KismetSystemLibrary.PrintText` (`|FormatText` "Current Pv : {CurrentPv} \nMax Pv : {MaxPv} \nCurrentXp : {CurrentXp} \nXp Need : {XpNeed} \nLevel : {Level} \nMax Level : {MaxLevel} \nStrenght : {Strength} \nBaseDamage : {BaseDamage} \nArmor : {Armor} \nVitality : {Vitality} \nCurrent Stamina : {CurrentStamina} \nMax Stamina : {MaxStamina} \nAssignment Point : {AssignmentPoint} \n" _currentpv _maxpv _currentxp _xpneed _level _maxlevel _strength _basedamage _armor _vitality _currentstamina _maxstamina _assignmentpoint) true true (struct :`G` 0.66 :`B` 1.0 :`A` 1.0) 10.0))

(fn `SaveMaxPv`
  (returns (OldMaxPv :type "Float (double-precision)"))
  (return (`.MaxPv_7_C8AB5A71489D35F3081461989E3096F6` (break `/Game/StarWarsCore/Blueprints/ActorsComponents/ManagerStats/Data/S_Stats` (`self.S_Stats`)))))

(fn `SetXpNeed`
  (params (Amount :type "Float (double-precision)"))
  (setmembers `/Game/StarWarsCore/Blueprints/ActorsComponents/ManagerStats/Data/S_Stats` :`StructRef` (`self.S_Stats`) :`XpNeed` (`KismetMathLibrary.FClamp` Amount 0.0 99999999.0)))

(fn `StrengthModifier`
  (params (Amount :type "Float (double-precision)") (Add :type Boolean))
  (if Add
    (`self.AddToStrength`)
    (else
      (`self.SubstractToStrength`))))

(fn `StrengthSet`
  (params (Amount :type "Float (double-precision)"))
  (setmembers `/Game/StarWarsCore/Blueprints/ActorsComponents/ManagerStats/Data/S_Stats` :`StructRef` (`self.S_Stats`) :`Strength` (`KismetMathLibrary.FClamp` Amount 0.0 9999999.0)))

(fn `VitalityApply`
  (bind _s_stats (`self.S_Stats`))
  (bind ((`MaxPv_7_C8AB5A71489D35F3081461989E3096F6` _maxpv) (`Vitality_28_97E612684821BF45F3641790379A02EB` _vitality)) (break `/Game/StarWarsCore/Blueprints/ActorsComponents/ManagerStats/Data/S_Stats` _s_stats))
  (setmembers `/Game/StarWarsCore/Blueprints/ActorsComponents/ManagerStats/Data/S_Stats` :`StructRef` _s_stats :`MaxPv` (+ _maxpv (* _vitality (`self.VitalityCoefficient`)))))

(fn `VitalityModifier`
  (params (Amount :type "Float (double-precision)") (Add :type Boolean))
  (if Add
    (`self.AddVitality`)
    (else
      (`self.SubstractVitality`))))

(fn `VitalitySet`
  (params (Amount :type "Float (double-precision)"))
  (setmembers `/Game/StarWarsCore/Blueprints/ActorsComponents/ManagerStats/Data/S_Stats` :`StructRef` (`self.S_Stats`) :`Vitality` (`KismetMathLibrary.FClamp` Amount 0.0 9999999.0)))