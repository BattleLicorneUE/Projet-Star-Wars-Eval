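; AC_ManagerExperience is an actor component that applies level-ups to the player character's AC_Stats component.
; LevelUp raises the level, updates max PV and required XP, then grants one assignment point.
; Below the max level, the DT_Leveling row named after the new level supplies max PV, and the following level's row supplies the XP needed.
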(event `LevelUp`
  (`self.LevelUpgrade`))

(fn `ChangePvAndXpInTermsOfLevel`
  (bind _returnvalue (`Actor.GetComponentByClass` (`GameplayStatics.GetPlayerCharacter` 0) "/Game/StarWarsCore/Blueprints/ActorsComponents/ManagerStats/AC_Stats.AC_Stats_C"))
  (bind ((`Level_14_AC96BB6B44E2483A794787BE8E04C43B` _level) (`MaxLevel_16_D89379EE46214A511074F2947D840039` _maxlevel)) (break `/Game/StarWarsCore/Blueprints/ActorsComponents/ManagerStats/Data/S_Stats` (`/Game/StarWarsCore/Blueprints/ActorsComponents/ManagerStats/AC_Stats.S_Stats` (`Actor.GetComponentByClass` (`GameplayStatics.GetPlayerCharacter` 0) "/Game/StarWarsCore/Blueprints/ActorsComponents/ManagerStats/AC_Stats.AC_Stats_C"))))
  (if (not (>= _level _maxlevel))
    (bind _returnvalue_2 (`|GetDataTableRow` "/Game/StarWarsCore/Blueprints/ActorsComponents/ManagerExperience/Data/DT_Leveling.DT_Leveling" (`KismetStringLibrary.Conv_StringToName` (`KismetStringLibrary.Conv_IntToString` _level)))
      (:`then`
        (message `/Game/StarWarsCore/Blueprints/ActorsComponents/ManagerStats/BPI_Stats.SetMaxPv` _returnvalue (`.TotalPvAfterLeveling_8_913B2A2C4E1C978EBAF7C4B48D156DF8` (break `/Game/StarWarsCore/Blueprints/ActorsComponents/ManagerExperience/Data/S_Leveling` _returnvalue_2)))
        (bind _returnvalue_3 (`|GetDataTableRow` "/Game/StarWarsCore/Blueprints/ActorsComponents/ManagerExperience/Data/DT_Leveling.DT_Leveling" (`KismetStringLibrary.Conv_StringToName` (`KismetStringLibrary.Conv_IntToString` (+ (`.Level_14_AC96BB6B44E2483A794787BE8E04C43B` (break `/Game/StarWarsCore/Blueprints/ActorsComponents/ManagerStats/Data/S_Stats` (`/Game/StarWarsCore/Blueprints/ActorsComponents/ManagerStats/AC_Stats.S_Stats` _returnvalue))) 1))))
          (:`then`
            (message `/Game/StarWarsCore/Blueprints/ActorsComponents/ManagerStats/BPI_Stats.XpNeedSet` (`Actor.GetComponentByClass` (`GameplayStatics.GetPlayerCharacter` 0) "/Game/StarWarsCore/Blueprints/ActorsComponents/ManagerStats/AC_Stats.AC_Stats_C") (`.XpNeed_6_D39A695B4C5AE51408E548A3D53A63BA` (break `/Game/StarWarsCore/Blueprints/ActorsComponents/ManagerExperience/Data/S_Leveling` _returnvalue_3)))))))))

(fn `LevelUpgrade`
  (bind _returnvalue (`Actor.GetComponentByClass` (`GameplayStatics.GetPlayerCharacter` 0) "/Game/StarWarsCore/Blueprints/ActorsComponents/ManagerStats/AC_Stats.AC_Stats_C"))
  (message `/Game/StarWarsCore/Blueprints/ActorsComponents/ManagerStats/BPI_Stats.ModifyLevel` _returnvalue 1 true)
  (`self.ChangePvAndXpInTermsOfLevel`)
  (message `/Game/StarWarsCore/Blueprints/ActorsComponents/ManagerStats/BPI_Stats.ModifyAssignmentPoint` _returnvalue 1.0 true))