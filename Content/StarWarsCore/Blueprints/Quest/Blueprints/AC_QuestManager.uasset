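; Quest manager component that holds the quest list and displays a quest in an on-screen quest bar.
; On BeginPlay it creates the W_QuestBar widget, adds it to the viewport and refreshes it with the first quest's name and first objective.
; A separate ResizeQuest function appends every QuestsData table row to the Quests array, but nothing in this graph calls it.
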(event `self.ReceiveBeginPlay`
  (bind _returnvalue (`|CreateWidget` "/Game/StarWarsCore/Blueprints/Quest/Blueprints/UI/W_QuestBar.W_QuestBar_C"))
  (bind _output_get (set `self.QuestBar` _returnvalue))
  (`UserWidget.AddToViewport` _output_get 0)
  (`self.UpdateQuestUI`))

(fn `ResizeQuest`
  (bind _questsdata (`self.QuestsData`))
  (bind _outrownames (`DataTableFunctionLibrary.GetDataTableRowNames` _questsdata))
  (for _array_element _outrownames
    (bind _returnvalue (`|GetDataTableRow` _questsdata _array_element)
      (:`then`
        (`KismetArrayLibrary.Array_Add` (`self.Quests`) _returnvalue)))))

(fn `UpdateQuestUI`
  (bind _w_questactive (`/Game/StarWarsCore/Blueprints/Quest/Blueprints/UI/W_QuestBar.W_QuestActive` (`self.QuestBar`)))
  (bind (_name _description _questtype _completed _objective) (break `/Game/StarWarsCore/Blueprints/Quest/Blueprints/S_Quest` (`|GetArrayItem` (`self.Quests`))))
  (`self.QuestBar`
    (:`then`
      (set `TextBlock.Text` (`KismetTextLibrary.Conv_NameToText` _name) (`/Game/StarWarsCore/Blueprints/Quest/Blueprints/UI/W_QuestActive.Name` _w_questactive))
      (set `TextBlock.Text` (`KismetTextLibrary.Conv_NameToText` (`.Name_2_02CD69F84CBEEEEAC8AD8FA2F0D4CE50` (break `/Game/StarWarsCore/Blueprints/Quest/Blueprints/S_Objective` (`|GetArrayItem` _objective)))) (`/Game/StarWarsCore/Blueprints/Quest/Blueprints/UI/W_QuestActive.Objective` _w_questactive)))
    (:`else`)))