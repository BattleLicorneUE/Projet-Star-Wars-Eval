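; Quest manager component that runs a linear sequence of quests loaded from a data table and shows the active one in a quest bar widget.
; UpdateQuest branches on Learn or Kill type, with Kill incrementing a count before both advance the objective.
; Passing the last objective index completes the quest, activates the next and rebuilds the UI.
; Debug keys print quest states or force an update.
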(event Custom|UpdateQuest
  ;[1 1 1] Update Quest
  (Utilities|QuestActive
    (:true
      (switch Utilities|FlowControl|Switch|SwitchonE_QuestType (Utilities|TypeQuest)
        (:NewEnumerator0
          (Player|ObjectiveComplete))
        (:NewEnumerator1
          (CallFunction|IncrementCount)
          (Player|ObjectiveComplete))))))

(event EventBeginPlay
  ;[0.2135 0.2135 0.2135] Create widget au begin play
  (bind _returnvalue (UserInterface|CreateWidget "/Game/StarWarsCore/Blueprints/Quest/Blueprints/UI/W_QuestBar.W_QuestBar_C"))
  (bind _output_get (Variables|Default|SetQuestBar _returnvalue))
  (UserInterface|Viewport|AddtoViewport _output_get 0)
  (Player|AddQuest)
  (Player|SetActiveQuest)
  (UI|UpdateQuestUI))

(event Input|KeyboardEvents|DebugKeyP
  (params (Key :type Key%20Structure :default "None") (ActionValue :type Input%20Action%20Value%20Structure))
  ;[1 1 1] Debug Keys
  (:Pressed
    (for _array_element (Variables|Default|GetQuests)
      (Development|PrintString (Utilities|String|Append (Utilities|String|ToString(Name) (.Name (Utilities|Struct|BreakS_Quest _array_element))) " : " (Utilities|String|ToString(Boolean) (.Completed (Utilities|Struct|BreakS_Quest _array_element))))))))

(event Input|KeyboardEvents|DebugKeyO
  (params (Key :type Key%20Structure :default "None") (ActionValue :type Input%20Action%20Value%20Structure))
  ;[1 1 1] Debug Keys
  (:Pressed
    (CallFunction|UpdateQuest)
    (Development|PrintString (Utilities|String|Append (Utilities|String|ToString(Integer) (Variables|Default|GetObjectiveIndex)) " " (Utilities|String|ToString(Integer) (Variables|Default|GetQuestindex))))
    (Development|PrintString (Utilities|String|ToString(Integer) (.Count (Utilities|Struct|BreakS_Objective (Utilities|Array|Get(acopy) (.Objective (Utilities|Struct|BreakS_Quest (Variables|Default|GetActiveQuest))) (Variables|Default|GetObjectiveIndex))))))))

(fn AddQuest
  (bind _questsdata (Variables|Default|GetQuestsData))
  (bind _outrownames (DataTable|GetDataTableRowNames _questsdata))
  (for _array_element _outrownames
    (bind _returnvalue (Utilities|GetDataTableRow _questsdata _array_element)
      (:then
        (Utilities|Array|Add (Variables|Default|GetQuests) _returnvalue)))))

(fn UpdateQuestUI
  (bind _questbar (Variables|Default|GetQuestBar))
  (bind _activequest (Variables|Default|GetActiveQuest))
  (bind (_name _description _questtype _completed _objective) (Utilities|Struct|BreakS_Quest _activequest))
  (bind _questbox (Variables|/Game/StarWarsCore/Blueprints/Quest/Blueprints/UI/W_QuestBar.W_QuestBar_C|GetQuestBox _questbar))
  (Variables|Default|GetQuestBar
    (:then
      (Widget|Panel|ClearChildren _questbox)
      (bind _returnvalue (UserInterface|CreateWidget "/Game/StarWarsCore/Blueprints/Quest/Blueprints/UI/W_QuestActive.W_QuestActive_C" 0 _activequest))
      (Widget|Panel|AddChild _questbox _returnvalue)
      (Variables|/Script/UMG.TextBlock|SetText (Variables|/Game/StarWarsCore/Blueprints/Quest/Blueprints/UI/W_QuestActive.W_QuestActive_C|GetName _returnvalue) (Utilities|Text|ToText(Name) _name))
      (Variables|/Script/UMG.TextBlock|SetText (Variables|/Game/StarWarsCore/Blueprints/Quest/Blueprints/UI/W_QuestActive.W_QuestActive_C|GetObjective _returnvalue) (Utilities|Text|ToText(Name) (.Name (Utilities|Struct|BreakS_Objective (Utilities|Array|Get(acopy) _objective (Variables|Default|GetObjectiveIndex)))))))
    (:else)))

(fn ObjectiveComplete
  (bind _quests (Variables|Default|GetQuests))
  (bind _questindex (Variables|Default|GetQuestindex))
  (bind _output (Utilities|Array|Get(acopy) _quests _questindex))
  (bind _objective (Utilities|Struct|BreakS_Quest _output))
  (if (>= (Variables|Default|GetObjectiveIndex) (Utilities|Array|Length _objective))
    (Utilities|Struct|SetmembersinS_Objective (Utilities|Array|Get(acopy) _objective (Variables|Default|GetObjectiveIndex)) true)
    (Player|QuestCompleted)
    (UI|UpdateQuestUI)
    (else
      (Utilities|Struct|SetmembersinS_Objective (Utilities|Array|Get(acopy) _objective (Variables|Default|GetObjectiveIndex)) true)
      (Variables|Default|SetObjectiveIndex (+ (Variables|Default|GetObjectiveIndex) 1)))))

(fn QuestCompleted
  (Utilities|Struct|SetmembersinS_Quest (Utilities|Array|Get(acopy) (Variables|Default|GetQuests) (Variables|Default|GetQuestindex)) true)
  (Variables|Default|SetQuestindex (+ (Variables|Default|GetQuestindex) 1))
  (Variables|Default|SetObjectiveIndex 0)
  (Player|SetActiveQuest))

(fn SetActiveQuest
  (Variables|Default|SetActiveQuest (Utilities|Array|Get(acopy) (Variables|Default|GetQuests) (Variables|Default|GetQuestindex))))

(fn IncrementCount
  (bind _activequest (Variables|Default|GetActiveQuest))
  (bind _objectiveindex (Variables|Default|GetObjectiveIndex))
  (bind _objective (Utilities|Struct|BreakS_Quest _activequest))
  (bind _output (Utilities|Array|Get(acopy) _objective _objectiveindex))
  (bind (_name _description _objectivecompleted _count _total) (Utilities|Struct|BreakS_Objective _output))
  (Utilities|Struct|SetmembersinS_Objective _output (+ _count 1))
  (if (== _count _total)
    (return)))