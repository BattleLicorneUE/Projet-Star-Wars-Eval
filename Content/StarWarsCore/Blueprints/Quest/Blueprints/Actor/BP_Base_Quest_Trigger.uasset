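; Base quest trigger actor that starts the quest named by its QuestID when the player character enters its box.
; It fires only while the player's AC_QuestManager has no active quest, and latches Activated once the quest starts.
; The QuestID enum string is the row name into the QuestData table; that row's index in the manager's Quests array sets the active quest and shows the quest bar.
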(event `self.ReceiveActorBeginOverlap`
  (params (OtherActor :type "Actor Object Reference")))

(event `self.Box.OnComponentBeginOverlap`
  (params (OverlappedComponent :type "PrimitiveComponent Object Reference") (OtherActor :type "Actor Object Reference") (OtherComp :type "PrimitiveComponent Object Reference") (OtherBodyIndex :type Integer) (bFromSweep :type Boolean) (SweepResult :type "HitResult Structure (by ref)"))
  (bind _returnvalue (`GameplayStatics.GetPlayerCharacter` 0))
  (bind _returnvalue_2 (`self.GetComponentByClass` _returnvalue "/Game/StarWarsCore/Blueprints/Quest/Blueprints/ActorComponents/AC_QuestManager.AC_QuestManager_C"))
  (bind _returnvalue_3 (`|GetEnumeratorNameAsString` (`self.QuestID`)))
  (if (not (`self.Activated?`))
    (if (== OtherActor _returnvalue)
      (bind _questactive_ (`/Game/StarWarsCore/Blueprints/Quest/Blueprints/ActorComponents/AC_QuestManager.IsQuestActive` _returnvalue_2))
      (if (not _questactive_)
        (`KismetSystemLibrary.PrintString` _returnvalue_3)
        (bind _returnvalue_4 (`|GetDataTableRow` "/Game/StarWarsCore/Blueprints/Quest/Blueprints/Data/QuestData.QuestData" (`KismetStringLibrary.Conv_StringToName` _returnvalue_3))
          (:`then`
            (`/Game/StarWarsCore/Blueprints/Quest/Blueprints/ActorComponents/AC_QuestManager.SetActiveQuest` _returnvalue_2 (`KismetArrayLibrary.Array_Find` (`/Game/StarWarsCore/Blueprints/Quest/Blueprints/ActorComponents/AC_QuestManager.Quests` _returnvalue_2) _returnvalue_4))
            (`/Game/StarWarsCore/Blueprints/Quest/Blueprints/ActorComponents/AC_QuestManager.DisplayQuestBar` _returnvalue_2)
            (set `self.Activated?` true)))))))

(fn `UserConstructionScript`)